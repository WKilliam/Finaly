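; PC_UnitController is a controller Blueprint that handles the fire input for the controlled hero unit.
; Pressing OpenFire casts the pawn to BpCharacter_UnitHero and continues only when its current movement acceleration is zero, so movement input blocks shooting.
; It then casts the WeaponPosition child actor to the pistol Blueprint and calls OpenFire on it, so other weapon classes do not fire.
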(event EventBeginPlay)

(event EventTick
  (params (DeltaSeconds :type Float%20%28single-precision%29)))

(event Input|ActionEvents|InputActionOpenFire
  (params (Key :type Key%20Structure :default "None"))
  (:Pressed
    (bind _asbp_character_unit_hero (Utilities|Casting|CastToBpCharacter_UnitHero (Pawn|GetControlledPawn)))
    (if (not (!= (Math|Vector|VectorLength (Pawn|Components|CharacterMovement|GetCurrentAcceleration (Variables|/Script/Engine.Character|GetCharacterMovement _asbp_character_unit_hero))) 0.0))
      (bind _asbp_actor_unit_weapon_pistol (Utilities|Casting|CastToBpActor_UnitWeapon_Pistol (Variables|/Script/Engine.ChildActorComponent|GetChildActor (Variables|/Game/Finaly/Core/Character/BpCharacter_Unit.BpCharacter_Unit_C|GetWeaponPosition _asbp_character_unit_hero))))
      (Default|OpenFire _asbp_actor_unit_weapon_pistol))))

(fn ConstructionScript)